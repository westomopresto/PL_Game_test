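; Player pawn Blueprint that makes post-process fog respond to the position of the lantern it carries.
; On BeginPlay it creates a dynamic instance of M_Fog_Simple and assigns it, alongside MI_3DFog, to the first PostProcessVolume found, with brightness limits pinned for fixed exposure.
; Every Tick it writes the lantern's world location into the material's LightWorldPosition parameter, so the fog follows the light.
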(event `Initialize Fog`
  (bind (_returnvalue_x _returnvalue_y _returnvalue_z) (`KismetMathLibrary.BreakVector` (`SceneComponent.K2_GetComponentLocation` (`self.BP_Lantern`))))
  ;[1 1 1 1 50] This was created with Austin for look deving light and fog as it applies to materials. This assigns the material that was created to the BP_Lantern.
  (bind _outactors (`GameplayStatics.GetAllActorsOfClass` "/Script/Engine.PostProcessVolume"))
  (set `self.PPV` (`|GetArrayItem` _outactors))
  (bind _returnvalue (`KismetMaterialLibrary.CreateDynamicMaterialInstance` "/Game/Plaguelands/MasterMaterials/Fog/M_Fog_Simple.M_Fog_Simple"))
  (bind _output_get (set `self.Fog_Material` _returnvalue))
  (set `PostProcessVolume.Settings` (make `PostProcessSettings` :`AutoExposureMinBrightness` 1.0 :`AutoExposureMaxBrightness` 1.0 :`WeightedBlendables` (make `WeightedBlendables` (`|MakeArray` (make `WeightedBlendable` 1.0 _output_get) (make `WeightedBlendable` 1.0 "/Game/Plaguelands/Assets/VFX/Fog/MI_3DFog.MI_3DFog")))) (`self.PPV`))
  (`MaterialInstanceDynamic.SetVectorParameterValue` (`self.Fog_Material`) "LightWorldPosition" (make `LinearColor` _returnvalue_x _returnvalue_y _returnvalue_z 1.0)))

(event `self.ReceiveBeginPlay`
  ;[1 1 1 1 50] Human Player-Only Stuff
  (`parent.ReceiveBeginPlay`)
  (`self.Initialize Fog`))

(event `self.ReceiveTick`
  (params (DeltaSeconds :type "Float (single-precision)"))
  (bind (_returnvalue_x _returnvalue_y _returnvalue_z) (`KismetMathLibrary.BreakVector` (`SceneComponent.K2_GetComponentLocation` (`self.BP_Lantern`))))
  ;[1 1 1 1 50] Comment
  (`parent.ReceiveTick` DeltaSeconds)
  (`MaterialInstanceDynamic.SetVectorParameterValue` (`self.Fog_Material`) "LightWorldPosition" (make `LinearColor` _returnvalue_x _returnvalue_y _returnvalue_z 1.0)))

(fn `UserConstructionScript`)