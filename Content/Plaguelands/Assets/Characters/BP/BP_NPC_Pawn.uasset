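; NPC pawn for Plaguelands: an AI-driven character that starts equipped with a hammer and drops its equipped weapons on death.
; On BeginPlay it creates and starts an StMc_Behavior_Base state machine with itself as context, then grants and selects the starter weapon.
; Walk speed is adjusted every tick.
; Death shuts down the state machine, clears AI focus and spawns each weapon's item at the pawn's location before running parent logic.
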(event `self.ReceiveTick`
  (params (DeltaSeconds :type "Float (single-precision)"))
  (`parent.ReceiveTick` DeltaSeconds)
  (`self.Adjust WalkSpeed`))

(event `self.Died`
  ;[1 1 1] New Ai State machine stuff
  (`SMInstance.Shutdown` (`self.Our_StateMachine`))
  (`AIController.K2_ClearFocus` (`AIBlueprintHelperLibrary.GetAIController` self))
  ;;[1 1 1] Drop items on death
  (for _array_element (`self.Equipped Weapons`)
    (`|SpawnActorFromClass` (`.Class_23_5E4612AF4A2209A0F55239BA2590A084` (break `/Game/Plaguelands/BP/Inventory_System/STR_Item` (`.ItemStruct_23_97225A8C43069BC5D5AB60B9F8339523` (break `/Game/Plaguelands/BP/Inventory_System/STR_Weapon` (`/Game/Plaguelands/BP/Inventory_System/Weapon_Object.Weapon Struct` _array_element))))) (`KismetMathLibrary.Conv_VectorToTransform` (`self.K2_GetActorLocation`)) "Undefined" "OverrideRootScale" null null))
  (`parent.Died`))

(event `self.ReceiveBeginPlay`
  ;[1 1 1] New Ai State machine stuff
  (`parent.ReceiveBeginPlay`)
  (`self.Initialize AI`)
  (`self.Starter_Weapons` (`|MakeArray` "/Game/Plaguelands/BP/Item_Pickups/Weapons/BP_Hammer_Item.BP_Hammer_Item_C" :!type "/Game/Plaguelands/BP/Item_Pickups/BP_Item_Equipment_Base Class Reference"))
  (`self.Switch Weapons` 0))

(event `Initialize AI`
  ;[1 1 1] New Ai State machine stuff
  (bind _output_get (set `self.Our_StateMachine` (`SMBlueprintUtils.CreateStateMachineInstance` "/Game/Plaguelands/BP/AI_Support/State_Machines/StMc_Behavior_Base.StMc_Behavior_Base_C" self)))
  (`SMInstance.Start` _output_get))

(fn `UserConstructionScript`
  (`parent.UserConstructionScript`))