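; Base Blueprint for interactable item containers in Plaguelands, each with its own inventory component.
; BeginPlay turns the InitialContents map of item classes and quantities into slot structs, copying them by index into the component's inventory.
; Interact stores the interacting BP_Player_Pawn and toggles the inventory.
; CloseContainer toggles it again and clears that player's InteractedContainer reference, if both are valid.
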(event `Close Container`
  (bind _interacted_player (`self.Interacted Player`))
  ;[1 1 1] Comment
  (`/Engine/EditorBlueprintResources/StandardMacros.IsValid` _interacted_player
    (:`Is Valid`
      (`/Engine/EditorBlueprintResources/StandardMacros.IsValid` (`/Game/Plaguelands/Assets/Characters/BP/BP_Character_Base.InteractedContainer` _interacted_player)
        (:`Is Valid`
          (`/Game/Plaguelands/BP/Inventory_System/BP_Inventory_Component.Toggle_Inventory` (`self.BP_Inventory_Component`))
          (set `/Game/Plaguelands/Assets/Characters/BP/BP_Character_Base.InteractedContainer` null _interacted_player))))))

(event `/Game/Plaguelands/BP/Inventory_System/BP_Interact_Interface.Interact`
  (params (Interactor :type "Actor Object Reference"))
  ;[1 1 1 1 20] This is making it so whenever the player uses the interact interface with a container object, it will cast to the BP_ThirdPersonPlayer to get access to something (not sure what at this point). It then calls the Toggle Inventory Function that was created in the BP_Inventory_Component. This effectively opens the inventory of any container when the player invokes the interact event.
  (bind _asbp_player_pawn (cast `/Game/Plaguelands/Assets/Characters/BP/BP_Player_Pawn` Interactor))
  (set `self.Interacted Player` _asbp_player_pawn)
  (`/Game/Plaguelands/BP/Inventory_System/BP_Inventory_Component.Toggle_Inventory` (`self.BP_Inventory_Component`)))

(event `self.ReceiveBeginPlay`
  ;[1 1 1 1 20] This is copying the predefined contents to be set for the container into the item array of the BP_Inventory_Component.
  (bind _keys (`BlueprintMapLibrary.Map_Keys` (`self.Initial Contents`)))
  (for _array_element _keys
    (`KismetArrayLibrary.Array_Add` (`self.Items`) (make `/Game/Plaguelands/BP/Inventory_System/STR_Slot` (defaults `/Game/Plaguelands/BP/Item_Containers/BP_Container_Base` _array_element) (`BlueprintMapLibrary.Map_Find` (`self.Initial Contents`) _array_element)))
    (`self.Add STR Slots to Inventory`)))

(event `Add STR Slots to Inventory`
  ;[1 1 1 1 20] This is copying the predefined contents to be set for the container into the item array of the BP_Inventory_Component.
  (for (_array_element _array_index) (`self.Items`)
    (`KismetArrayLibrary.Array_Set` (`/Game/Plaguelands/BP/Inventory_System/BP_Inventory_Component.Inventory` (`self.BP_Inventory_Component`)) _array_index _array_element true)))

(fn `UserConstructionScript`)