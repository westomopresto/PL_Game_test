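; BP_PatrolPath is a spline-based actor that defines a patrol path in the world, filed under AI world context support.
; The construction script sets the spline open or looped from the ClosedLoop variable, and BeginPlay caches the total SplineLength.
; GetLocationAlongSpline converts a distance along the spline into a world-space location.
; The actor itself contains no movement or AI logic.
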(event `self.ReceiveBeginPlay`
  (set `self.SplineLength` (`SplineComponent.GetSplineLength` (`self.Spline`))))

(fn `Get Location along Spline`
  (params (Distance :type "Float (double-precision)"))
  (returns (ReturnValue :type "Vector Structure"))
  (return (`SplineComponent.GetLocationAtDistanceAlongSpline` (`self.Spline`) Distance "World")))

(fn `UserConstructionScript`
  (`SplineComponent.SetClosedLoop` (`self.Spline`) (`self.Closed Loop?`) true))