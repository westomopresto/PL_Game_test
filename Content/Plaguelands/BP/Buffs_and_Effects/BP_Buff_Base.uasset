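; Base buff actor that temporarily scales one attribute on its owning character for a set duration.
; On BeginPlay with a valid owner, RenewBuff saves the current value from the ActiveAttributes map, multiplies it by AttributeModifier and starts a retriggerable delay.
; Repeated renewals restart the timer but also re-save and re-multiply the already modified value.
; ClearBuff restores the saved value, leaves the owner's Buffs and destroys the actor.
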(event `Attribute Manipulate`
  (bind _active_attributes (`/Game/Plaguelands/Assets/Characters/BP/BP_Character_Base.Active_Attributes` (`self.Owning Character`)))
  (bind _value (`BlueprintMapLibrary.Map_Find` _active_attributes (`self.Attribute Changed`)))
  (set `self.Original Attribute Untouched` _value)
  (`BlueprintMapLibrary.Map_Add` _active_attributes (`self.Attribute Changed`) (* _value (`self.Attribute Modifier`))))

(event `self.ReceiveBeginPlay`
  ;[1 1 1] Begin Play
  (`/Engine/EditorBlueprintResources/StandardMacros.IsValid` (`self.Owning Character`)
    (:`Is Valid`
      (`self.Renew Buff`))))

(event `Renew Buff`
  ;[1 1 1] Buff
  (`self.Attribute Manipulate`)
  ;[1 1 1] After Buff duration, revert attirubtes & remove buff
  (`KismetSystemLibrary.RetriggerableDelay` (`self.Duration`))
  (`self.Clear Buff`))

(event `Clear Buff`
  (bind _owning_character (`self.Owning Character`))
  ;[1 1 1] Clear buff
  (`BlueprintMapLibrary.Map_Add` (`/Game/Plaguelands/Assets/Characters/BP/BP_Character_Base.Active_Attributes` _owning_character) (`self.Attribute Changed`) (`self.Original Attribute Untouched`))
  (`KismetArrayLibrary.Array_RemoveItem` (`/Game/Plaguelands/Assets/Characters/BP/BP_Character_Base.Buffs` _owning_character) self)
  (`self.K2_DestroyActor`))

(fn `UserConstructionScript`)