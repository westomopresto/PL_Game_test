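; Base spell actor that casts as soon as it spawns, launching projectiles and playing a cast sound.
; BeginPlay stores the spell's transform, then CastSuccess spawns the configured number of projectiles there and calls CastFX for the sound.
; Each projectile always spawns regardless of collision, inherits the spell's owner and instigator, and receives a reference to the spell that cast it.
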(event `Cast FX`
  (`GameplayStatics.PlaySoundAtLocation` "/Game/Test/sarmy_Test/Assets/Sounds/Footsteps_A_11.Footsteps_A_11" (`self.K2_GetActorLocation`) (struct) 1.0 1.0 0.0 null null null))

(event `Cast Success`
  (`self.Spawn Projectiles Function` (`self.Projectile Class`) (`self.Projectile Quantity`) (`self.Projectile Spawn Transform`))
  (`self.Cast FX`))

(event `self.ReceiveBeginPlay`
  (set `self.Projectile Spawn Transform` (`self.GetTransform`))
  (`self.Cast Success`))

(fn `Spawn Projectiles Function`
  (params (`Spawn Class` :type "/Game/Plaguelands/BP/Projectiles/BP_Projectile_Base Class Reference") (Quantity :type Integer) (SpawnTransform :type "Transform Structure"))
  ;[1 1 1] How many copies of this projectile do we spawn?
  (for _ (range Quantity)
    ;[1 1 1] Spawns the Projectile actors
    (`|SpawnActorFromClass` `Spawn Class` SpawnTransform "AlwaysSpawn" "OverrideRootScale" (`self.GetOwner`) 0.0 self 500.0 (`self.GetInstigator`)))
  (return))

(fn `UserConstructionScript`)