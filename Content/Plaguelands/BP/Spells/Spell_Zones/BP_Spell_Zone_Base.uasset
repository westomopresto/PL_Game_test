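; Base actor for spell zones that apply a buff to any character inside their sphere.
; The zone scales up on spawn and, if Duration is positive, waits that long before scaling again and destroying itself.
; Overlap begin and every Tick clear any same-class buff and spawn a fresh, short-lived one attached to the character, so the effect persists while inside.
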(event `Apply Effects`
  (params (`Base Character` :type "/Game/Plaguelands/Assets/Characters/BP/BP_Character_Base Object Reference"))
  ;[0.7823 0.3958 1] Check if there's a buff of the same type on the character, if so, delete it and reapply a fresh one, if not apply a fresh one
  (bind (_buff_already_applied _if_true___applied_buff) (`self.Duplicate Buff Check` `Base Character` (`self.Buff to Apply`)))
  (if _buff_already_applied
    ;;[1 1 1] Renew buff instead of applying a new one
    (`/Game/Plaguelands/BP/Buffs_and_Effects/BP_Buff_Base.Clear Buff` _if_true___applied_buff))
  (bind _returnvalue (`|SpawnActorFromClass` (`self.Buff to Apply`) (`self.GetTransform` `Base Character`) "AlwaysSpawn" "OverrideRootScale" `Base Character` 0.25 "NewEnumerator3" `Base Character` 0.25 `Base Character`))
  (`KismetArrayLibrary.Array_Add` (`/Game/Plaguelands/Assets/Characters/BP/BP_Character_Base.Buffs` `Base Character`) _returnvalue)
  (`self.K2_AttachToActor` _returnvalue `Base Character` "None" "KeepWorld" "KeepWorld" "KeepWorld" true))

(event `Character in Zone`
  (params (`Other Actor` :type "Object Object Reference"))
  ;[1 1 1] Only apply to characters
  (bind _asbp_character_base (cast `/Game/Plaguelands/Assets/Characters/BP/BP_Character_Base` `Other Actor`))
  (`self.Apply Effects` _asbp_character_base))

(event `Spawn Effects`
  ;[1 1 1] Spawn Effects (happens before post spawn
  (bind (_direction _scale_alpha) (`Timeline|Grow` :!via `PlayFromStart`)
    (:`Update`
      (`self.SetActorScale3D` (`KismetMathLibrary.Conv_DoubleToVector` _scale_alpha)))
    (:`Finished`
      (`self.Post Spawn Effects`))))

(event `Post Spawn Effects`
  (bind _duration (`self.Duration`))
  ;[1 1 1] Post Spawn Effects
  (if (> _duration 0.0)
    (`KismetSystemLibrary.Delay` _duration)
    (bind (_direction _scale_alpha) (`Timeline|Scale size and destroy` :!via `PlayFromStart`)
      (:`Update`
        (`self.SetActorScale3D` (`KismetMathLibrary.Conv_DoubleToVector` _scale_alpha)))
      (:`Finished`
        (`self.K2_DestroyActor`)))))

(event `self.ReceiveBeginPlay`
  ;[0 1 0.1047] Begin Play
  (`self.Spawn Effects`))

(event `self.ReceiveActorBeginOverlap`
  (params (OtherActor :type "Actor Object Reference"))
  (`self.Character in Zone` OtherActor))

(event `self.ReceiveTick`
  (params (DeltaSeconds :type "Float (single-precision)"))
  (for _array_element (`PrimitiveComponent.GetOverlappingActors` (`self.Sphere`) "/Game/Plaguelands/Assets/Characters/BP/BP_Character_Base.BP_Character_Base_C")
    (`self.Character in Zone` _array_element)))

(fn `Duplicate Buff Check`
  (params (`Base Character` :type "/Game/Plaguelands/Assets/Characters/BP/BP_Character_Base Object Reference") (`Buff Class` :type "/Game/Plaguelands/BP/Buffs_and_Effects/BP_Buff_Base Class Reference"))
  (returns (`Buff already Applied` :type Boolean) (`if true - Applied Buff` :type "/Game/Plaguelands/BP/Buffs_and_Effects/BP_Buff_Base Object Reference"))
  (for _array_element (`/Game/Plaguelands/Assets/Characters/BP/BP_Character_Base.Buffs` `Base Character`)
    (if (== `Buff Class` (`GameplayStatics.GetObjectClass` _array_element))
      (return true _array_element)))
  (return false null))

(fn `UserConstructionScript`)