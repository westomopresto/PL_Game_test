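; Inventory component that stores items in a fixed-size slot array and toggles the inventory window on the player's HUD canvas.
; PrepareInventory sizes the array and refreshes item data from class defaults on BeginPlay and whenever the window opens.
; AddToInventory tops up partial stacks or fills empty slots, with AddToStack passing any overflow back recursively.
; InventoryQuery checks whether the total held of an item class meets a requested amount.
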(event `self.ReceiveBeginPlay`
  (`self.Prepare_Inventory`))

(fn `Add_To_Inventory`
  (params (Content_To_Add :type "/Game/Plaguelands/BP/Inventory_System/STR_Slot Structure"))
  (returns (Success :type Boolean))
  (locals (IsSuccessful :type Boolean))
  ;[1 1 1 1 25] The "Add_to_Inventory" function is first checking to see if the item is stackable or not.
  (if (`.Stackable_5_19AF6C804206D92E87A6D9BD6BF40D35` (break `/Game/Plaguelands/BP/Inventory_System/STR_Item` (break `/Game/Plaguelands/BP/Inventory_System/STR_Slot` Content_To_Add)))
    ;;[1 1 1] This is using a macro that we create, called "Has Partial Stack". If the item is stackable, the picked up item is added to an existing stack (if one exists) or just makes a new stack if one does not. This is done via the "Add_to_Stack" function.
    (bind _stackindex (`self.Has_Partial_Stack` (`local.Content_To_Add`))
      (:`True`
        (bind _success (`self.Add_To_Stack` (`local.Content_To_Add`) _stackindex))
        (set `local.IsSuccessful` _success))
      (:`False`
        ;;[1 1 1] If it isn't stackable, it creates the item via the "Create Stack" function. Note that to get the variables for "Content to Add" you'll need to pull off from the pin and choose "Get Content to Add". This is because the pin of the function was originally split and can no longer be dragged from.
        (bind _success_2 (`self.Create_Stack` (`local.Content_To_Add`) :!label _label))
        (set `local.IsSuccessful` _success_2)))
    (else
      (goto _label)))
  (return (`local.IsSuccessful`)))

(fn `Add_To_Stack`
  (params (STR_Slot :type "/Game/Plaguelands/BP/Inventory_System/STR_Slot Structure") (Slot_Index :type Integer))
  (returns (Success :type Boolean))
  (locals (Current_Quantity :type Integer))
  (bind _inventory (`self.Inventory`))
  (bind _slot_index (`local.Slot_Index`))
  (bind (_str_slot_itemstored _str_slot_itemquantity _str_slot_equipped _str_slot_weaponobject) (break `/Game/Plaguelands/BP/Inventory_System/STR_Slot` (`local.STR_Slot`)))
  (bind (_str_slot_itemstored_2 _str_slot_itemquantity_2 _str_slot_equipped_2 _str_slot_weaponobject_2) (break `/Game/Plaguelands/BP/Inventory_System/STR_Slot` (`local.STR_Slot`)))
  (bind (_str_slot_itemstored_3 _str_slot_itemquantity_3) (break `/Game/Plaguelands/BP/Inventory_System/STR_Slot` (`local.STR_Slot`)))
  (bind (_name _description _cost _thumbnail _stackable _maxstacksize) (break `/Game/Plaguelands/BP/Inventory_System/STR_Item` _str_slot_itemstored))
  (bind _output (`|GetArrayItem` (`self.Inventory`) Slot_Index))
  (bind (_output_itemstored _output_itemquantity _output_equipped _output_weaponobject) (break `/Game/Plaguelands/BP/Inventory_System/STR_Slot` (`|GetArrayItem` _inventory _slot_index)))
  ;[1 1 1 1 15] This is adding the amount of an item picked up to the amount the player already has in their inventory. This is done to check whether the items go into an existying stack or have to make a new one.
  (bind _output_get (set `local.Current_Quantity` (`.ItemQuantity_7_2566D49B444A6F65D1E8BDB2690FDED1` (break `/Game/Plaguelands/BP/Inventory_System/STR_Slot` _output))))
  (if (> (+ _output_get (`.ItemQuantity_7_2566D49B444A6F65D1E8BDB2690FDED1` (break `/Game/Plaguelands/BP/Inventory_System/STR_Slot` STR_Slot))) (`.MaxStackSize_17_2739BDD04A2A93DDF3D8DC8DC771708E` (break `/Game/Plaguelands/BP/Inventory_System/STR_Item` (break `/Game/Plaguelands/BP/Inventory_System/STR_Slot` _output))))
    ;[1 1 1] This is filling up the rest of the current stack. Note that there is going to be an excess of said item after this is complete.
    (`KismetArrayLibrary.Array_Set` (`self.Inventory`) (`local.Slot_Index`) (make `/Game/Plaguelands/BP/Inventory_System/STR_Slot` _str_slot_itemstored _maxstacksize _str_slot_equipped _str_slot_weaponobject))
    ;[1 1 1] This is calling the "Add to Inventory" function again. This is essentially taking the overflow from the previous addition and placing it into a new slot.
    (`self.Add_To_Inventory` (make `/Game/Plaguelands/BP/Inventory_System/STR_Slot` _str_slot_itemstored_2 (- _str_slot_itemquantity_2 (- _maxstacksize (`local.Current_Quantity`))) _str_slot_equipped_2 _str_slot_weaponobject_2))
    (else
      ;[1 1 1] If the previous check is false, that means that the addition of the newly picked up item along with the previously stored amount of item are less than the max stack size. If that's the case, the "Array Element" is set for the inventory "Slot Index" and the picked up item(s) are added to the current slot of items.
      (`KismetArrayLibrary.Array_Set` _inventory _slot_index (make `/Game/Plaguelands/BP/Inventory_System/STR_Slot` _output_itemstored (+ _output_itemquantity _str_slot_itemquantity_3) _output_equipped _output_weaponobject))))
  (return true))

(fn `Create_Stack`
  (params (Content_To_Add :type "/Game/Plaguelands/BP/Inventory_System/STR_Slot Structure"))
  (returns (Success :type Boolean))
  (locals (HasSpace :type Boolean))
  (bind _inventory (`self.Inventory`))
  ;[1 1 1 1 25] This function finds an empty slot and fills it with the item(s) picked up.
  ;;[1 1 1 1 20] This is testing how many empty slots we have. If it's false, then the local variable, Has Space is always false and no stacks get made.
  (for _array_element (`self.Inventory`)
    (if (<= (`.ItemQuantity_7_2566D49B444A6F65D1E8BDB2690FDED1` (break `/Game/Plaguelands/BP/Inventory_System/STR_Slot` _array_element)) 0)
      (set `local.HasSpace` true)
      (break)))
  ;;[1 1 1 1 20] Once the loop is broken, it does a check of Has Space, and if that's been set, we create a new stack.
  (if (`local.HasSpace`)
    ;;[1 1 1 1 20] This is the part where a new stack is created.
    (`KismetArrayLibrary.Array_Set` _inventory (`KismetArrayLibrary.Array_Find` _inventory (make `/Game/Plaguelands/BP/Inventory_System/STR_Slot` (struct :`Name` "NSLOCTEXT(\"[888389C84EE88BD84E3BC797EAC25BC3]\", \"776F414544DD2BFF5C3298AB300C95E2\", \"None\")" :`Description` "NSLOCTEXT(\"[888389C84EE88BD84E3BC797EAC25BC3]\", \"49EBF4E141396BB4072CDBA37C6B8D28\", \"None\")" :`Stackable` true :`MaxStackSize` 5 :`Consumable` true :`ItemType` "NewEnumerator2"))) (`local.Content_To_Add`))
    (return (`local.HasSpace`))
    (else
      (return false))))

(fn `Inventory_Query`
  (params (QueryItem :type "/Game/Plaguelands/BP/Item_Pickups/BP_Item_Base Class Reference") (QueryAmount :type Integer))
  (returns (IsInInventory :type Boolean))
  (locals (RunningTotal :type Integer))
  ;[1 1 1 1 20] Note that this is the player's inventory array.
  (for _array_element (`self.Inventory`)
    (if (== (`.Class_23_5E4612AF4A2209A0F55239BA2590A084` (break `/Game/Plaguelands/BP/Inventory_System/STR_Item` (break `/Game/Plaguelands/BP/Inventory_System/STR_Slot` _array_element))) (`local.QueryItem`))
      (set `local.RunningTotal` (+ (`.ItemQuantity_7_2566D49B444A6F65D1E8BDB2690FDED1` (break `/Game/Plaguelands/BP/Inventory_System/STR_Slot` _array_element)) (`local.RunningTotal`)))))
  (return (>= (`local.RunningTotal`) (`local.QueryAmount`))))

(fn `Prepare_Inventory`
  ;[1 1 1 1 25] This will set the number of slots for the inventory array with the NumberOfSlots variable. By default, the array is empty. This isbasically resizing the inventory based on number of items.
  (`KismetArrayLibrary.Array_Resize` (`self.Inventory`) (`self.NumberOfSlots`))
  ;[1 1 1 1 25] Comment
  ;;[1 1 1 1 20] This is checking each item to see if its class has been set. That is the condition of the Branch.
  (for (_array_element _array_index) (`self.Inventory`)
    (bind (_name _description _cost _thumbnail _stackable _maxstacksize _consumable _durability _class) (break `/Game/Plaguelands/BP/Inventory_System/STR_Item` (break `/Game/Plaguelands/BP/Inventory_System/STR_Slot` _array_element)))
    ;;[1 1 1 1 20] This then sets the array element for the inventory.
    (if (!= _class null)
      (`KismetArrayLibrary.Array_Set` (`self.Inventory`) _array_index (make `/Game/Plaguelands/BP/Inventory_System/STR_Slot` (defaults `/Game/Plaguelands/BP/Inventory_System/BP_Inventory_Component` _class) (`.ItemQuantity_7_2566D49B444A6F65D1E8BDB2690FDED1` (break `/Game/Plaguelands/BP/Inventory_System/STR_Slot` _array_element)) (`.Equipped_9_4D37CF064719B5F14E9EA5B4100081A4` (break `/Game/Plaguelands/BP/Inventory_System/STR_Slot` _array_element)) (`.WeaponObject_14_DC5351C2463FB3B616B83096F59FD8D2` (break `/Game/Plaguelands/BP/Inventory_System/STR_Slot` _array_element)))))))

(fn `Toggle_Inventory`
  ;[1 1 1 1 50] Function for Toggle Inventory works based off of a Valid Check. If the window isn't open, the check is invalid, and so it creates the Inventory UI. If the Check is valid, the Inventory UI is open, and so it closes
  (if (`self.WindowOpen?`)
    ;;[1 1 1 1 25] Closes Inventory UI and returns focus to the game.
    (`Widget.RemoveFromParent` (`self.InventoryWindow`))
    (set `self.InventoryWindow` null)
    (`WidgetBlueprintLibrary.SetInputMode_GameOnly` (`GameplayStatics.GetPlayerController` 0))
    (set `self.WindowOpen?` false)
    (else
      ;;[1 1 1 1 25] Opens Inventory UI and sets focus to game and UI.
      (`self.Prepare_Inventory`)
      (bind _returnvalue (`|CreateWidget` "/Game/Plaguelands/BP/Inventory_System/Inventory_UI/Inventory_Window.Inventory_Window_C" null self))
      (set `self.InventoryWindow` _returnvalue)
      (bind _asbp_player_controller (cast `/Game/Plaguelands/BP/BP_PlayerController` (`GameplayStatics.GetPlayerController` 0)))
      (bind _returnvalue_2 (`CanvasPanel.AddChildToCanvas` (`/Game/Plaguelands/UI/HUD/HUD.HUD_Canvas` (`/Game/Plaguelands/BP/BP_PlayerController.HUD_Widget` _asbp_player_controller)) (`self.InventoryWindow`)))
      ;;;[1 1 1 1 25] Autosizes the window. Not sure to what?
      (`CanvasPanelSlot.SetAutoSize` _returnvalue_2 true)
      ;;;[1 1 1 1 25] Setting alignment, anchors, and position for the Inventory Window.
      (`CanvasPanelSlot.SetAlignment` _returnvalue_2 (0.5 0.5))
      (`CanvasPanelSlot.SetAnchors` _returnvalue_2 (make `Anchors` (0.5 0.5) (0.5 0.5)))
      (`CanvasPanelSlot.SetPosition` _returnvalue_2 (`self.Position`))
      ;;;[1 1 1 1 25] Sets the input mode to both the game and UI so the user can interact with the game as well as the UI elements. Need to disable movement when the UI is open.
      (`WidgetBlueprintLibrary.SetInputMode_GameAndUIEx` (`GameplayStatics.GetPlayerController` 0) (`self.InventoryWindow`) "DoNotLock" false)
      (set `self.WindowOpen?` true))))