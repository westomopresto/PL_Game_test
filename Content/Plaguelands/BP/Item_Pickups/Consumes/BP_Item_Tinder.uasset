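; BP_Item_Tinder is a consumable tinder pickup that refuels the player's lantern when used.
; Its UseItem override runs the parent logic, then casts player character 0 to BP_Player_Pawn and reaches the BP_Lantern through the pawn's child actor component.
; It calls AddFuel with the FuelPickupAmount variable and returns true once both casts succeed.
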(fn `Use_Item`
  (returns (Success :type Boolean))
  (`parent.Use_Item`)
  ;[1 1 1 1 25] This is the custom part of the tinder use function. It's first casting to the BP_ThirdPersonPlayer and getting the Player Character. This allows for getting the component in the Player Character that has the BP_Lantern. The BP_Lantern needs to be converted to a child actor and then can be piped into a cast to the BP_Lantern Class. From there, Use the "Add Fuel" function (the amount it increments is based on the number we place in the input value we assigned within the custom function. In this case, it was promoted to a variable.
  (bind _asbp_player_pawn (cast `/Game/Plaguelands/Assets/Characters/BP/BP_Player_Pawn` (`GameplayStatics.GetPlayerCharacter` 0)))
  (bind _asbp_lantern (cast `/Game/Plaguelands/BP/Lantern/BP_Lantern` (`ChildActorComponent.ChildActor` (`/Game/Plaguelands/Assets/Characters/BP/BP_Player_Pawn.BP_Lantern` _asbp_player_pawn))))
  (`/Game/Plaguelands/BP/Lantern/BP_Lantern.AddFuel` _asbp_lantern (`self.Fuel_Pickup_Amount`))
  (return true))

(fn `UserConstructionScript`
  (`parent.UserConstructionScript`))