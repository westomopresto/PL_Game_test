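; Base melee weapon Blueprint that plays the owner's attack montage on fire and damages what its blade hits.
; StartMelee and StopMelee toggle a per-tick hurtbox that capsule-traces between top and bottom points at the last and interpolated halfway positions, covering gaps between frames.
; Each new non-owner hit spawns VFX and sound, damages BP_Character_Base, fires a hit dispatcher and knocks Characters back.
; A per-swing hit list prevents repeat hits.
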(event `self.Press Weapon Fire`
  (`parent.Press Weapon Fire`)
  (`/Game/Plaguelands/Assets/Characters/BP/BP_Character_Base.MeleeAttackMontage` (`self.OwningCharacter`) "/Game/Plaguelands/Assets/Characters/Animation/Biped/Retargeted/ATART_Retarget/Montages/Doc_2hand_Attack.Doc_2hand_Attack" "attackStart")
  (`KismetSystemLibrary.PrintString` "Fire weapon" true true (struct :`R` 1.0 :`G` 0.864192 :`A` 1.0)))

(event `HitSomething`
  (params (DamageDealt :type "Float (double-precision)") (ActorHit :type "Actor Object Reference") (HitLocation :type "Vector Structure"))
  (`self.HitSomethingDispatcher_0` DamageDealt ActorHit HitLocation (`self.SwingThrough?`)))

(event `Start Melee`
  (`KismetArrayLibrary.Array_Clear` (`self.Collected_Hits`))
  (set `self.Hurtbox_Active` true)
  (set `self.LastTop` (`SceneComponent.K2_GetComponentLocation` (`self.hit_top`)))
  (set `self.LastBottom` (`SceneComponent.K2_GetComponentLocation` (`self.hit_bottom`))))

(event `self.ReceiveTick`
  (params (DeltaSeconds :type "Float (single-precision)"))
  (bind _returnvalue (`SceneComponent.K2_GetComponentLocation` (`self.hit_bottom`)))
  (bind _returnvalue_2 (`SceneComponent.K2_GetComponentLocation` (`self.hit_top`)))
  ;[1 1 1] Only traces if the "hurtbox" bool is active
  (if (`self.Hurtbox_Active`)
    ;[1 1 1] Initial trace for the frame
    (`|ExecutionSequence`
      (:`then_0`
        (bind (_outhit _returnvalue_3) (`self.TraceHitPoints` (`self.LastTop`) (`self.LastBottom`) (struct :`R` 1.0 :`G` 1.0 :`A` 1.0) (struct :`G` 1.0 :`B` 0.069863 :`A` 1.0) true))
        (`self.ApplyDamageToHits` _outhit _returnvalue_3))
      (:`then_1`
        ;[1 1 1] Does a second trace between the last trace, and the current trace
        (bind (_outhit_2 _returnvalue_4) (`self.TraceHitPoints` (`KismetMathLibrary.VLerp` (`self.LastTop`) _returnvalue_2 0.5) (`KismetMathLibrary.VLerp` (`self.LastBottom`) _returnvalue 0.5) (struct :`R` 0.968277 :`G` 1.0 :`A` 1.0) (struct :`R` 1.0 :`G` 0.080432 :`A` 1.0) true))
        (`self.ApplyDamageToHits` _outhit_2 _returnvalue_4)
        ;;[1 1 1] This sets the initial location for the next time we trace (next frame)
        (set `self.LastTop` _returnvalue_2)
        (set `self.LastBottom` _returnvalue)))))

(event `Stop Melee`
  (set `self.Hurtbox_Active` false))

(event `self.ReceiveBeginPlay`
  (bind _returnvalue (`self.GetParentActor`))
  ;[1 1 1] If this weapon was a child of an enemy/player/character, set owner variable to that
  (`/Engine/EditorBlueprintResources/StandardMacros.IsValid` _returnvalue
    (:`Is Valid`
      (`self.SetOwner` _returnvalue))))

(fn `ApplyDamageToHits`
  (params (`Hit Result` :type "HitResult Structure") (ValidHit :type Boolean))
  (locals (`Hit Actor` :type "Actor Object Reference") (`Impact Point` :type "Vector Structure" :default (0.0 0.0 0.0)))
  (bind (_bblockinghit _binitialoverlap _time _distance _location _impactpoint _normal _impactnormal _physmat _hitactor) (`GameplayStatics.BreakHitResult` `Hit Result`))
  (bind _impact_point (`local.Impact Point`))
  (bind _hit_actor (`local.Hit Actor`))
  (bind _damage (`self.Damage`))
  (bind _returnvalue (`self.K2_GetActorLocation` (`self.GetOwner`)))
  (bind _returnvalue_2 (`self.K2_GetActorLocation` (`local.Hit Actor`)))
  (set `local.Hit Actor` _hitactor)
  (set `local.Impact Point` _impactpoint)
  (if ValidHit
    (if (!= (`self.GetOwner`) (`local.Hit Actor`))
      (`|ExecutionSequence`
        (:`then_0`
          ;[1 1 1] Did we already hit this?
          (if (`KismetArrayLibrary.Array_Contains` (`self.Collected_Hits`) (`local.Hit Actor`))
            ;[1 1 1] Actor already in our list, do nothing and return out
            (return)
            (else
              ;[1 1 1] OKAY do damage
              (`|ExecutionSequence`
                (:`then_0`
                  ;;[1 1 1] VFX & SFX
                  (`GameplayStatics.SpawnEmitterAtLocation` "/Game/Plaguelands/Assets/VFX/Particles/P_ImpactA_01_Blue_Edit.P_ImpactA_01_Blue_Edit" _impact_point (struct) (0.5 0.5 0.5))
                  (`GameplayStatics.PlaySoundAtLocation` "/Game/UE4_Packs/MegaBundleSoundPack/PhobiaSoundPack/Audio/Cue/book_wav_Cue.book_wav_Cue" _impact_point (struct) 1.0 (`KismetMathLibrary.RandomFloatInRange` 1.5 2.0) 0.0 "/Game/Test/sarmy_Test/Assets/Sounds/Damage_Attenuation.Damage_Attenuation" null null))
                (:`then_1`
                  ;;[1 1 1] Actual damage events/etc
                  (`self.Deal Damage to Character` (`local.Hit Actor`) _damage)
                  (`self.HitSomething` _damage (`local.Hit Actor`) (`local.Impact Point`))
                  (`/Engine/EditorBlueprintResources/StandardMacros.IsValid` _hit_actor
                    (:`Is Valid`
                      (bind _ascharacter (cast `Character` _hit_actor))
                      (`Character.LaunchCharacter` _ascharacter (* (`KismetMathLibrary.Normal` (`KismetMathLibrary.MakeVector` (.x (`KismetMathLibrary.GetDirectionUnitVector` _returnvalue _returnvalue_2)) (.y (`KismetMathLibrary.GetDirectionUnitVector` _returnvalue _returnvalue_2)) (+ (.z (`KismetMathLibrary.GetDirectionUnitVector` _returnvalue _returnvalue_2)) 2.0))) (`self.KnockbackPower`)) false false)
                      (`KismetSystemLibrary.DrawDebugArrow` _returnvalue _returnvalue_2 50.0 (struct :`R` 1.0 :`G` 1.0 :`B` 1.0 :`A` 1.0) 1.0 10.0))))))))
        (:`then_1`
          ;[1 1 1] Add the hit actor to our list
          (`KismetArrayLibrary.Array_AddUnique` (`self.Collected_Hits`) (`local.Hit Actor`))))
      (else
        (return)))
    (else
      (return))))

(fn `Deal Damage to Character`
  (params (InputPin :type "Actor Object Reference") (BaseDamage :type "Float (double-precision)"))
  (bind _asbp_character_base (cast `/Game/Plaguelands/Assets/Characters/BP/BP_Character_Base` InputPin))
  (`GameplayStatics.ApplyDamage` _asbp_character_base BaseDamage null self))

(fn `TraceHitPoints`
  (params (First :type "Vector Structure") (End :type "Vector Structure") (TraceColor :type "LinearColor Structure") (TraceHitColor :type "LinearColor Structure") (`CapsuleTrace?` :type Boolean) (DrawDebugType :type "EDrawDebugTrace Enum" :default "None"))
  (returns (OutHit :type "HitResult Structure") (ReturnValue :type Boolean))
  (bind _array (`|MakeArray` "ObjectTypeQuery7" "ObjectTypeQuery3" "ObjectTypeQuery1" :!type "EObjectTypeQuery Enum"))
  (bind _array_2 (`|MakeArray` (`self.GetOwner`)))
  (if `CapsuleTrace?`
    (bind (_outhit _returnvalue) (`KismetSystemLibrary.CapsuleTraceSingleForObjects` First End (`self.HurtBoxRadius`) 5.0 _array false _array_2 DrawDebugType true TraceColor TraceHitColor 3.0))
    (return _outhit _returnvalue)
    (else
      (bind (_outhit_2 _returnvalue_2) (`KismetSystemLibrary.LineTraceSingleForObjects` First End _array false _array_2 DrawDebugType true TraceColor TraceHitColor 3.0))
      (return _outhit_2 _returnvalue_2))))

(fn `UserConstructionScript`)