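; Base ranged weapon for Plaguelands, set up as a chargeable bow that fires projectiles.
; Pressing fire plays the bow montage and starts charging, while releasing plays its shoot section at double speed and cancels the charge.
; Release then scales projectile speed and damage by ChargeAmount, spawns the configured projectile class at BarrelExit and prints the charge for debugging.
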(event `Bow Charge`
  (`|PlayMontage` (`self.Weapon_Skeletal_Mesh`) "/Game/Plaguelands/Assets/Weapons/SkinnedMeshes/Bow/Animations/bow_montage.bow_montage" 1.0 0.0 "Default"
    (:`then`
      (`self.Charge` 1.0))))

(event `self.Press Weapon Fire`
  (`parent.Press Weapon Fire`)
  (`self.Bow charge`))

(event `self.Release Weapon Fire`
  (`parent.Release Weapon Fire`)
  (`self.Bow Release`))

(event `Bow Release`
  (`|PlayMontage` (`self.Weapon_Skeletal_Mesh`) "/Game/Plaguelands/Assets/Weapons/SkinnedMeshes/Bow/Animations/bow_montage.bow_montage" 2.0 0.0 "bow_shoot"
    (:`then`
      (`self.Cancel Charge`)
      (`self.Shoot Projectile` (`KismetMathLibrary.Lerp` 400.0 2000.0 (/ (`self.ChargeAmount`) 100.0)) (* (`self.Damage`) (/ (`self.ChargeAmount`) 100.0)))
      (`KismetSystemLibrary.PrintString` (`KismetStringLibrary.Conv_DoubleToString` (`self.ChargeAmount`))))))

(fn `Shoot Projectile`
  (params (`Projectile Speed` :type "Float (double-precision)") (`Impact Damage` :type "Float (double-precision)"))
  (bind _asbp_projectile_base (castclass `/Game/Plaguelands/BP/Projectiles/BP_Projectile_Base` (`self.Projectile Class`)))
  (`|SpawnActorFromClass` _asbp_projectile_base (`SceneComponent.K2_GetComponentToWorld` (`self.BarrelExit`)) "Undefined" "OverrideRootScale" null `Impact Damage` null `Projectile Speed` null))

(fn `UserConstructionScript`
  (`parent.UserConstructionScript`))