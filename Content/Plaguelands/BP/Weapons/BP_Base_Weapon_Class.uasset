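; BP_Base_Weapon_Class is a base weapon Blueprint that provides shared charge and unsheathe behavior, with empty press and release fire events.
; Charge scales a timeline's play rate by the given charge time to ramp ChargeAmount from 0 to 100, and CancelCharge stops it.
; Unsheathe plays a sound and spawns an attached dust emitter at the root component, both using footstep assets.
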(event `Charge`
  (params (`Charge Time` :type "Float (double-precision)" :default 1.0))
  ;[1 1 1] Charge - Behaviors
  (`TimelineComponent.SetPlayRate` (`self.ChargeTimeline`) (/ 1.0 `Charge Time`))
  (bind (_direction _alpha) (`Timeline|ChargeTimeline` :!via `PlayFromStart` :!label _label)
    (:`Update`
      (set `self.ChargeAmount` (`KismetMathLibrary.Lerp` 0.0 100.0 _alpha)))))

(event `Cancel Charge`
  ;[1 1 1] Charge - Behaviors
  (goto _label :!via `Stop`))

(event `Press Weapon Fire`)

(event `Release Weapon Fire`)

(event `Unsheathe`
  (`self.Play Unsheathe Sound` 1.0)
  (`self.Spawn Unsheathe VFX`))

(fn `Play Unsheathe Sound`
  (params (PitchMultiplier :type "Float (double-precision)" :default 1.0))
  (`GameplayStatics.PlaySoundAtLocation` "/Game/Test/sarmy_Test/Assets/Sounds/Footsteps_A_5.Footsteps_A_5" (`SceneComponent.K2_GetComponentLocation` (`self.DefaultSceneRoot`)) (struct) 1.0 PitchMultiplier 0.0 "/Game/Test/sarmy_Test/Assets/Sounds/Character_Att.Character_Att" null null)
  (return))

(fn `Spawn Unsheathe VFX`
  (`GameplayStatics.SpawnEmitterAttached` "/Game/Test/Weston_Test/Effects/Particle_Systems/P_Dust_Footstep.P_Dust_Footstep" (`self.DefaultSceneRoot`))
  (return))

(fn `UserConstructionScript`)