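; Base projectile Blueprint that damages what it hits, crediting the instigator's controller and owning spell, and ignores its instigator while moving.
; Sphere hits apply damage and play sound and emitter effects after a short retriggerable delay; the overlap handler is unwired.
; It expires on first impact or when movement stops, depending on StopOnFirstImpact, driving its scale by timeline before destroying itself.
; Construction sets initial speed from ProjectileSpeed.
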(event `On Impact FX`
  (params (`Impact Location` :type "Vector Structure"))
  ;[0.3761 0.5616 1] FX &/or Sound Effects to trigger on impact
  (`KismetSystemLibrary.RetriggerableDelay` 0.1)
  (`GameplayStatics.PlaySoundAtLocation` (`self.Impact Sound`) `Impact Location` (struct) 1.0 1.0 0.0 null null null)
  (`GameplayStatics.SpawnEmitterAtLocation` (`self.Impact Emitter`) `Impact Location` (struct) (`self.Impact Emitter Scale`)))

(event `self.Sphere.OnComponentHit`
  (params (HitComponent :type "PrimitiveComponent Object Reference") (OtherActor :type "Actor Object Reference") (OtherComp :type "PrimitiveComponent Object Reference") (NormalImpulse :type "Vector Structure") (Hit :type "HitResult Structure (by ref)"))
  ;[1 1 1] On hit or overlap, trigger impact events
  (`self.Impact Events` OtherActor Hit))

(event `self.ReceiveBeginPlay`
  ;[1 0.8266 0] ignores player's collider when we spawn this projectile
  (`PrimitiveComponent.IgnoreActorWhenMoving` (`self.Sphere`) (`self.Instigator`) true))

(event `Damage Sequence`
  (params (DamagedActor :type "Actor Object Reference"))
  ;[1 0.4478 0.2729] Damage logic
  (`GameplayStatics.ApplyDamage` DamagedActor (`self.Impact Damage`) (`self.GetInstigatorController`) (`self.Owning Spell`)))

(event `self.Sphere.OnComponentBeginOverlap`
  (params (OverlappedComponent :type "PrimitiveComponent Object Reference") (OtherActor :type "Actor Object Reference") (OtherComp :type "PrimitiveComponent Object Reference") (OtherBodyIndex :type Integer) (bFromSweep :type Boolean) (SweepResult :type "HitResult Structure (by ref)"))
  ;[1 1 1] On hit or overlap, trigger impact events
)

(event `Impact Events`
  (params (DamagedActor :type "Actor Object Reference") (Hit :type "HitResult Structure (by ref)"))
  (bind (_bblockinghit _binitialoverlap _time _distance _location _impactpoint) (`GameplayStatics.BreakHitResult` Hit))
  ;[1 1 1] Sequence of events after projectile impacts something or someone
  (`self.Damage Sequence` DamagedActor)
  (`self.On Impact FX` _impactpoint)
  (if (`self.Stop on first impact?`)
    (`self.Impact Complete` _impactpoint)))

(event `Impact Complete`
  (params (`Impact Location` :type "Vector Structure"))
  ;[0 1 0.2293] Impact Completed event
  (`self.Expire`))

(event `Expire`
  ;[1 0 0] Expire
  (bind (_direction _scale_alpha) (`Timeline|Timeline_0` :!via `PlayFromStart`)
    (:`Update`
      (`self.SetActorScale3D` (`KismetMathLibrary.Conv_DoubleToVector` _scale_alpha)))
    (:`Finished`
      (`self.K2_DestroyActor`))))

(event `self.ProjectileMovement.OnProjectileStop`
  (params (ImpactResult :type "HitResult Structure (by ref)"))
  ;[1 1 1] Sequence of events after projectile impacts something or someone
  (if (not (`self.Stop on first impact?`))
    (`self.Impact Complete` (`.ImpactPoint` (`GameplayStatics.BreakHitResult` ImpactResult)))))

(fn `UserConstructionScript`
  (set `ProjectileMovementComponent.InitialSpeed` (`self.Projectile Speed`) (`self.ProjectileMovement`)))